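; Animation Modifier that bakes a FootOffset curve into an Animation Sequence from ball_l and ball_r motion.
; ExportMoveCurve samples component-space bone height per frame, zeroes frames below minimum plus tolerance, and normalizes each lift against its peak, writing per-bone _Height curves.
; MergeMoveCurve combines both feet, with non-zero right-foot values overriding the left.
; The raw-height exporter, ExportBoneHeight, is only called from disconnected nodes.
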(event `self.OnApply`
  (params (AnimationSequence :type "AnimSequence Object Reference"))
  (`self.MergeMoveCurve` AnimationSequence 0.75 (`|MakeArray` "ball_l" "ball_r" :!type "Name") "FootOffset"))

(fn `ExportBoneHeight`
  (params (AnimSequence :type "AnimSequence Object Reference") (BoneName :type Name))
  (locals (theFrame :type Integer) (thePose :type "Transform Structure") (theKeys :type "Array of Float (double-precision)") (theTimes :type "Array of Float (double-precision)") (theCurveName :type Name))
  (set `local.theCurveName` (`KismetStringLibrary.Conv_StringToName` (`KismetStringLibrary.Concat_StrStr` (`KismetStringLibrary.Conv_NameToString` (`local.BoneName`)) "_Height")))
  (`|ExecutionSequence`
    (:`then_0`
      (bind _returnvalue (`AnimationBlueprintLibrary.DoesCurveExist` (`local.AnimSequence`) (`local.theCurveName`) "RCT_Float"))
      (if _returnvalue
        (`AnimationBlueprintLibrary.RemoveCurve` (`local.AnimSequence`) (`local.theCurveName`))))
    (:`then_1`
      (`AnimationBlueprintLibrary.AddCurve` (`local.AnimSequence`) (`local.theCurveName`))
      (for _index (range (+ (`AnimationBlueprintLibrary.GetNumFrames` (`local.AnimSequence`)) 1))
        (set `local.theFrame` _index)
        (bind _returnvalue_2 (`VAT_Bone.GetBoneTransformCS` (`local.AnimSequence`) (`KismetMathLibrary.Conv_IntToBool` 0) (`local.theFrame`) (`local.BoneName`)))
        (set `local.thePose` _returnvalue_2)
        (`KismetArrayLibrary.Array_Add` (`local.theKeys`) (.z (.location (`local.thePose`))))
        (`KismetArrayLibrary.Array_Add` (`local.theTimes`) (`AnimationBlueprintLibrary.GetTimeAtFrame` (`local.AnimSequence`) (`local.theFrame`))))
      (`AnimationBlueprintLibrary.AddFloatCurveKeys` (`local.AnimSequence`) (`local.theCurveName`) (`local.theTimes`) (`local.theKeys`)))))

(fn `ExportMoveCurve`
  (params (AnimSequence :type "AnimSequence Object Reference") (BoneName :type Name) (OutputCurve :type Name) (Tolerance :type "Float (double-precision)" :default 0.5))
  (returns (OutputKeys :type "Array of Float (double-precision)") (OutputTimes :type "Array of Float (double-precision)"))
  (locals (theFrame :type Integer) (thePose :type "Transform Structure") (theKeys :type "Array of Float (double-precision)") (theTimes :type "Array of Float (double-precision)") (theCurveName :type Name) (OutputKyes :type Boolean) (theMinValue :type "Float (double-precision)" :default 0.0) (theStartIndex :type Integer) (theValue :type "Float (double-precision)") (theFinalIndex :type Integer) (theMaxRangeValue :type "Float (double-precision)") (theMatching :type Boolean :default false) (theMinRangeValue :type "Float (double-precision)" :default 0.0) (theOutputKeys :type "Array of Float (double-precision)") (theOutputTimes :type "Array of Float (double-precision)") (theOutputTime :type "Float (double-precision)") (theOutputValue :type "Float (double-precision)" :default 0.0) (theApexIndex :type Integer))
  (set `local.theCurveName` OutputCurve)
  (`|ExecutionSequence`
    (:`then_0`
      (if (not (== (`local.theCurveName`) "None"))
        (bind _returnvalue (`AnimationBlueprintLibrary.DoesCurveExist` (`local.AnimSequence`) (`local.theCurveName`) "RCT_Float"))
        (if _returnvalue
          (`AnimationBlueprintLibrary.RemoveCurve` (`local.AnimSequence`) (`local.theCurveName`)))
        (`AnimationBlueprintLibrary.AddCurve` (`local.AnimSequence`) (`local.theCurveName`))))
    (:`then_1`
      (for _index (range (+ (`AnimationBlueprintLibrary.GetNumFrames` (`local.AnimSequence`)) 1))
        (set `local.theFrame` _index)
        (bind _returnvalue_2 (`VAT_Bone.GetBoneTransformCS` (`local.AnimSequence`) (`KismetMathLibrary.Conv_IntToBool` 0) (`local.theFrame`) (`local.BoneName`)))
        (set `local.thePose` _returnvalue_2)
        (`KismetArrayLibrary.Array_Add` (`local.theKeys`) (.z (.location (`local.thePose`))))
        (`KismetArrayLibrary.Array_Add` (`local.theTimes`) (`AnimationBlueprintLibrary.GetTimeAtFrame` (`local.AnimSequence`) (`local.theFrame`))))
      (set `local.theMinValue` (`.MinValue` (`KismetMathLibrary.MinOfFloatArray` (`local.theKeys`))))
      (set `local.theMinRangeValue` (+ (`local.theMinValue`) (`local.Tolerance`)))
      (for (_array_element _array_index) (`local.theKeys`)
        (set `local.theValue` _array_element)
        (set `local.theStartIndex` _array_index)
        (set `local.theMatching` (>= (`local.theValue`) (`local.theMinRangeValue`)))
        (`|ExecutionSequence`
          (:`then_0`
            (if (`local.theMatching`)
              (`/Engine/EditorBlueprintResources/StandardMacros.DoOnce` false :!label _label
                (:`Completed`
                  (set `local.theMaxRangeValue` 0.0)
                  (for _index_2 (range (`local.theStartIndex`) (`KismetArrayLibrary.Array_Length` (`local.theKeys`)))
                    (bind _output (`|GetArrayItem` (`local.theKeys`) _index_2))
                    (if (>= _output (`local.theMinRangeValue`))
                      (if (>= _output (`local.theMaxRangeValue`))
                        (set `local.theMaxRangeValue` _output)
                        (set `local.theApexIndex` _index_2))
                      (else
                        (set `local.theFinalIndex` _index_2)
                        (break))))))
              (else
                (goto _label :!via `Reset`))))
          (:`then_1`
            (set `local.theOutputValue` (`KismetMathLibrary.SelectFloat` (`KismetMathLibrary.Abs` (/ (- (`local.theValue`) (`local.theMinRangeValue`)) (- (`local.theMaxRangeValue`) (`local.theMinRangeValue`)))) 0.0 (`local.theMatching`)))
            (set `local.theOutputTime` (`|GetArrayItem` (`local.theTimes`) (`local.theStartIndex`)))
            (`KismetArrayLibrary.Array_Add` (`local.theOutputKeys`) (`local.theOutputValue`))
            (`KismetArrayLibrary.Array_Add` (`local.theOutputTimes`) (`local.theOutputTime`))
            (if (not (== (`local.theCurveName`) "None"))
              (`AnimationBlueprintLibrary.AddFloatCurveKey` (`local.AnimSequence`) (`local.theCurveName`) (`local.theOutputTime`) (`local.theOutputValue`))))))
      (return (`local.theOutputKeys`) (`local.theOutputTimes`)))))

(fn `MergeMoveCurve`
  (params (AnimSequence :type "AnimSequence Object Reference") (Tolerance :type "Float (double-precision)" :default 0.75) (BonesName :type "Array of Name") (OutputCurve :type Name))
  (locals (theKeys :type "Array of Float (double-precision)") (theTimes :type "Array of Float (double-precision)") (MergeKeys :type "Array of Float (double-precision)") (MergeTimes :type "Array of Float (double-precision)"))
  (for _array_element BonesName
    (bind (_outputkeys _outputtimes) (`self.ExportMoveCurve` (`local.AnimSequence`) _array_element (`KismetStringLibrary.Conv_StringToName` (`KismetStringLibrary.Concat_StrStr` (`KismetStringLibrary.Conv_NameToString` _array_element) "_Height")) (`local.Tolerance`)))
    (set `local.theKeys` _outputkeys)
    (set `local.theTimes` _outputtimes)
    (if (== (`KismetArrayLibrary.Array_Length` (`local.MergeKeys`)) 0)
      (set `local.MergeKeys` (`local.theKeys`))
      (set `local.MergeTimes` (`local.theTimes`))
      (else
        (for (_array_element_2 _array_index) (`local.theKeys`)
          (if (!= _array_element_2 0.0)
            (`KismetArrayLibrary.Array_Set` (`local.MergeKeys`) _array_index (`|GetArrayItem` (`local.theKeys`) _array_index)))))))
  (bind _returnvalue (`AnimationBlueprintLibrary.DoesCurveExist` (`local.AnimSequence`) (`local.OutputCurve`) "RCT_Float"))
  (if _returnvalue
    (`AnimationBlueprintLibrary.RemoveCurve` (`local.AnimSequence`) (`local.OutputCurve`)))
  (`AnimationBlueprintLibrary.AddCurve` (`local.AnimSequence`) (`local.OutputCurve`))
  (`AnimationBlueprintLibrary.AddFloatCurveKeys` (`local.AnimSequence`) (`local.OutputCurve`) (`local.MergeTimes`) (`local.MergeKeys`)))