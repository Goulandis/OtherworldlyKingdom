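; BP_Cow is a cow actor that randomly varies its animation.
; On BeginPlay it caches its skeletal mesh's Anim_Cow instance and starts a looping timer that fires every few seconds.
; Each tick of the timer randomly either resets the anim instance's Index to zero and randomizes X, or assigns a random Index, leaving state selection to the animation Blueprint.
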(event `self.ReceiveBeginPlay`
  (bind _asanim_cow (cast `/Game/FarmAnimalsPack/Cow/Meshes/Anim_Cow` (`SkeletalMeshComponent.GetAnimInstance` (`self.SkeletalMesh`))))
  (set `self.AnimInstance` _asanim_cow)
  (`KismetSystemLibrary.K2_SetTimerDelegate` (delegate `CowAnim`) 5.0 true))

(event `CowAnim`
  (bind _returnvalue (`KismetMathLibrary.RandomIntegerInRange` -2 2))
  (bind _animinstance (`self.AnimInstance`))
  (if (<= _returnvalue 0)
    (set `/Game/FarmAnimalsPack/Cow/Meshes/Anim_Cow.Index` 0 _animinstance)
    (set `/Game/FarmAnimalsPack/Cow/Meshes/Anim_Cow.X` (`KismetMathLibrary.Conv_IntToDouble` (`KismetMathLibrary.RandomIntegerInRange` -2 2)) (`self.AnimInstance`))
    (else
      (set `/Game/FarmAnimalsPack/Cow/Meshes/Anim_Cow.Index` _returnvalue _animinstance))))

(fn `UserConstructionScript`)