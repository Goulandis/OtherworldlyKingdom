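; BP_Chicken is a farm animal chicken that varies its animation at random over time.
; On BeginPlay it casts the skeletal mesh's anim instance to Anim_Chicken and starts a looping timer.
; Each timer tick sets the anim instance's X and Y to new random normalized values, leaving the animation blueprint to turn them into poses.
; It has no movement, overlap or per-frame logic.
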(event `self.ReceiveBeginPlay`
  (bind _asanim_chicken (cast `/Game/FarmAnimalsPack/Chicken/Meshes/Anim_Chicken` (`SkeletalMeshComponent.GetAnimInstance` (`self.SkeletalMesh`))))
  (set `self.AnimInstance` _asanim_chicken)
  (`KismetSystemLibrary.K2_SetTimerDelegate` (delegate `ChickenAction`) 5.0 true))

(event `ChickenAction`
  (bind _animinstance (`self.AnimInstance`))
  (set `/Game/FarmAnimalsPack/Chicken/Meshes/Anim_Chicken.X` (`KismetMathLibrary.RandomFloatInRange` 0.0 1.0) _animinstance)
  (set `/Game/FarmAnimalsPack/Chicken/Meshes/Anim_Chicken.Y` (`KismetMathLibrary.RandomFloatInRange` 0.0 1.0) _animinstance))

(event `self.ReceiveTick`
  (params (DeltaSeconds :type "Float (single-precision)")))

(fn `UserConstructionScript`)